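; BP_Camera is a spring-arm camera rig that rotates from horizontal and vertical values passed in by a caller.
; Its custom event CE_相机旋转 (camera rotation) scales both values by a shared multiplier, adding yaw to the SpringArm's relative rotation.
; It then sets pitch separately, clamped just short of straight up and down to avoid flipping, while keeping roll and yaw.
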(event `CE_相机旋转`
  (params (`水平旋转` :type "Float (double-precision)") (`垂直旋转` :type "Float (double-precision)") (`旋转差值` :type "Float (double-precision)"))
  (bind _springarm (`self.SpringArm`))
  (`SceneComponent.K2_AddRelativeRotation` _springarm (`KismetMathLibrary.MakeRotator` 0.0 0.0 (* `水平旋转` `旋转差值`)) false false)
  (`SceneComponent.K2_SetRelativeRotation` _springarm (`KismetMathLibrary.MakeRotator` (.roll (`SceneComponent.RelativeRotation` _springarm)) (`KismetMathLibrary.FClamp` (+ (* `垂直旋转` `旋转差值`) (.pitch (`SceneComponent.RelativeRotation` _springarm))) -89.900002 89.900002) (.yaw (`SceneComponent.RelativeRotation` _springarm))) false false))

(event `self.ReceiveTick`
  (params (DeltaSeconds :type "Float (single-precision)")))

(fn `UserConstructionScript`)